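; BP_InteractiveTeleportChair is an interactive chair that teleports the player beside itself when activated.
; On BeginPlay it caches the first player's pawn as CurrentPlayer.
; The Activate event teleports that pawn to a fixed world-space offset from the chair's location, to the side and raised, keeping the pawn's current rotation.
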(event `self.ReceiveBeginPlay`
  (`parent.ReceiveBeginPlay`)
  (set `self.CurrentPlayer` (`GameplayStatics.GetPlayerPawn` 0)))

(event `self.Activate`
  (bind _currentplayer (`self.CurrentPlayer`))
  (`self.K2_TeleportTo` _currentplayer (+ (`self.K2_GetActorLocation`) (0.0 -200.0 150.0)) (`self.K2_GetActorRotation` _currentplayer)))

(fn `UserConstructionScript`
  (`parent.UserConstructionScript`))