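; Base pawn with mouse look and gaze-based interaction with BP_InteractiveBase actors.
; Each Tick, TimedGaze line-traces from the camera and starts a timer on a new focus, clearing it when gaze leaves interactive objects.
; On expiry, Interact calls Activate on the object.
; The instant BasicGaze alternative and the timer bar spawn are disconnected, though code to move and destroy the bar remains.
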(event `InputAxisKey|MouseX`
  (params (AxisValue :type "Float (single-precision)"))
  (`self.AddControllerYawInput` (* AxisValue (`self.Head Speed`))))

(event `self.ReceiveTick`
  (params (DeltaSeconds :type "Float (single-precision)"))
  (`self.TimedGaze`))

(event `InputAxisKey|MouseY`
  (params (AxisValue :type "Float (single-precision)"))
  (`self.AddControllerPitchInput` (* (* AxisValue -1.0) (`self.Head Speed`))))

(fn `BasicGaze`
  (bind (_bblockinghit _binitialoverlap _time _distance _location _impactpoint _normal _impactnormal _physmat _hitactor) (`GameplayStatics.BreakHitResult` (`self.LineTraceTemp`)))
  (if _bblockinghit
    (bind _asbp_interactive_base (cast `/Game/Blueprints/BP_InteractiveBase` _hitactor)
      (:`then`
        (set `self.InteractiveObject` _asbp_interactive_base)
        (if (not (== (`self.InteractiveObject`) (`self.FocusObject`)))
          (set `self.FocusObject` (`self.InteractiveObject`))
          (`self.Interact`)))
      (:`CastFailed`
        (set `self.InteractiveObject` null :!label _label)
        (set `self.FocusObject` null)))
    (else
      (goto _label))))

(fn `Interact`
  (bind _interactiveobject (`self.InteractiveObject`))
  (bind _timerbaractor (`self.TimerBarActor`))
  (`/Engine/EditorBlueprintResources/StandardMacros.IsValid` _interactiveobject
    (:`Is Valid`
      (`/Game/Blueprints/BP_InteractiveBase.Activate` _interactiveobject)
      (`/Engine/EditorBlueprintResources/StandardMacros.IsValid` _timerbaractor
        (:`Is Valid`
          (`self.K2_DestroyActor` _timerbaractor))))))

(fn `LineTraceTemp`
  (returns (OutHit :type "HitResult Structure"))
  (bind _camera (`self.Camera`))
  (bind _returnvalue (`SceneComponent.K2_GetComponentLocation` _camera))
  (bind _outhit (`KismetSystemLibrary.LineTraceSingle` _returnvalue (+ _returnvalue (* (`SceneComponent.GetForwardVector` _camera) (`self.trace_distance`))) "TraceTypeQuery1"))
  (return _outhit))

(fn `TimedGaze`
  (bind _timerbaractor (`self.TimerBarActor`))
  (bind _timerbaractor_2 (`self.TimerBarActor`))
  (bind (_bblockinghit _binitialoverlap _time _distance _location _impactpoint _normal _impactnormal _physmat _hitactor) (`GameplayStatics.BreakHitResult` (`self.LineTraceTemp`)))
  (if _bblockinghit
    (bind _asbp_interactive_base (cast `/Game/Blueprints/BP_InteractiveBase` _hitactor)
      (:`then`
        (set `self.InteractiveObject` _asbp_interactive_base)
        (if (not (== (`self.InteractiveObject`) (`self.FocusObject`)))
          (set `self.FocusObject` (`self.InteractiveObject`))
          (`KismetSystemLibrary.K2_ClearAndInvalidateTimerHandle` (`self.Timer`))
          (bind _returnvalue (`KismetSystemLibrary.K2_SetTimer` null "Interact" (`self.max_gaze_time`)))
          (set `self.Timer` _returnvalue)
          (`/Engine/EditorBlueprintResources/StandardMacros.IsValid` _timerbaractor_2
            (:`Is Valid`
              (`self.K2_SetActorLocation` _timerbaractor_2 (+ _impactpoint (0.0 0.0 150.0)) false false)))))
      (:`CastFailed`
        (set `self.InteractiveObject` null :!label _label)
        (set `self.FocusObject` null)
        (`KismetSystemLibrary.K2_ClearAndInvalidateTimerHandle` (`self.Timer`))
        (`/Engine/EditorBlueprintResources/StandardMacros.IsValid` _timerbaractor
          (:`Is Valid`
            (`self.K2_DestroyActor` _timerbaractor)))))
    (else
      (goto _label))))

(fn `UserConstructionScript`)